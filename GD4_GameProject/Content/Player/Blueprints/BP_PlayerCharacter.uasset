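; First-person player character for a timed investigation game, handling movement, sprint, crouch, interaction, object inspection and evidence collection.
; Tick runs a camera line trace that sets the BPI_Interactable target and prompt, and paces footstep sounds.
; Inspection attaches objects to the camera for rotation and photo capture of unique evidence into an inventory, restoring them on exit.
; A looping countdown updates the timer widget, intensifies music late and triggers game over.
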(event Custom|GameOver
  (bind _returnvalue (Game|GetPlayerController 0))
  (bind _charactermovement (Variables|Character|GetCharacterMovement))
  (if (not (Variables|Timer|GetIsGameOver))
    (Variables|Timer|SetIsGameOver true)
    (Utilities|Time|ClearTimerbyFunctionName 0 "CountdownTick")
    (Class|NavMovementInterface|StopActiveMovement _charactermovement)
    (Pawn|Components|CharacterMovement|DisableMovement _charactermovement)
    (bind _returnvalue_2 (UserInterface|CreateWidget "/Game/UI/WBP_GameOver.WBP_GameOver_C" _returnvalue))
    (bind _output_get (Variables|Timer|SetGameOverWidget _returnvalue_2))
    (UserInterface|Viewport|AddtoViewport _output_get 0)
    (Variables|/Script/Engine.PlayerController|SetbShowMouseCursor _returnvalue true)
    (Input|SetInputModeUIOnly _returnvalue _output_get "DoNotLock" false)))

(event Input|EnhancedActionEvents|EnhancedInputActionIA_Look
  (params (ActionValue :type Vector%202D%20Structure) (ElapsedSeconds :type Float%20%28double-precision%29) (TriggeredSeconds :type Float%20%28double-precision%29) (InputAction :type Input%20Action%20Object%20Reference :default "/Game/Player/Blueprints/Input/IA_Look.IA_Look"))
  ;[0.15 0.15 0.15 0.5] Look and Rotation Code
  (if (Variables|Interact|GetIsInspecting)
    (Utilities|IsValid (Variables|Inspect|GetInspectedObject)
      (:Is%20Valid
        (bind _output_get (Variables|Inspect|SetInspectYaw (+ (* (.x ActionValue) (Variables|Inspect|GetInspectRotationSpeed)) (Variables|Inspect|GetInspectYaw))))
        (bind _output_get_2 (Variables|Inspect|SetInspectPitch (+ (* (* (.y ActionValue) -1.0) (Variables|Inspect|GetInspectRotationSpeed)) (Variables|Inspect|GetInspectPitch))))
        (Transformation|SetActorRelativeRotation (Variables|Inspect|GetInspectedObject) (Math|Rotator|MakeRotator 0.0 _output_get_2 _output_get))))
    (else
      (Pawn|Input|AddControllerYawInput (.x ActionValue))
      (Pawn|Input|AddControllerPitchInput (* (.y ActionValue) -1.0)))))

(event Input|EnhancedActionEvents|EnhancedInputActionIA_Move
  (params (ActionValue :type Vector%202D%20Structure) (ElapsedSeconds :type Float%20%28double-precision%29) (TriggeredSeconds :type Float%20%28double-precision%29) (InputAction :type Input%20Action%20Object%20Reference :default "/Game/Player/Blueprints/Input/IA_Move.IA_Move"))
  (bind _returnvalue (Pawn|GetControlRotation :!class /Script/Engine.Pawn))
  (bind _yaw (Math|Rotator|BreakRotator _returnvalue))
  (bind _returnvalue_2 (Math|Rotator|MakeRotator 0.0 0.0 _yaw))
  ;[0.15 0.15 0.15 0.5] Movement forward and back and right and left
  (Pawn|Input|AddMovementInput (Math|Vector|GetForwardVector _returnvalue_2) (.y ActionValue) false)
  (Pawn|Input|AddMovementInput (Math|Vector|GetRightVector _returnvalue_2) (.x ActionValue) false))

(event Input|EnhancedActionEvents|EnhancedInputActionIA_Jump
  (params (ActionValue :type Boolean) (ElapsedSeconds :type Float%20%28double-precision%29) (TriggeredSeconds :type Float%20%28double-precision%29) (InputAction :type Input%20Action%20Object%20Reference :default "/Game/Player/Blueprints/Input/IA_Jump.IA_Jump"))
  ;[0.15 0.15 0.15 0.5] Jump Code
  (:Started
    (Character|Jump))
  (:Completed
    (Character|StopJumping)))

(event Input|EnhancedActionEvents|EnhancedInputActionIA_Crouch
  (params (ActionValue :type Boolean) (ElapsedSeconds :type Float%20%28double-precision%29) (TriggeredSeconds :type Float%20%28double-precision%29) (InputAction :type Input%20Action%20Object%20Reference :default "/Game/Player/Blueprints/Input/IA_Crouch.IA_Crouch"))
  ;[0.15 0.15 0.15 0.5] Crouch Code
  (:Started
    (Variables|Components|SetIsSprinting false)
    (Variables|/Script/Engine.CharacterMovementComponent|SetMaxWalkSpeed (Variables|Character|GetCharacterMovement) (Variables|Components|GetWalkSpeed))
    (Character|Crouch))
  (:Completed
    (Character|UnCrouch)
    (Variables|/Script/Engine.CharacterMovementComponent|SetMaxWalkSpeed (Variables|Character|GetCharacterMovement) (Variables|Components|GetWalkSpeed))))

(event Input|EnhancedActionEvents|EnhancedInputActionIA_Sprint
  (params (ActionValue :type Boolean) (ElapsedSeconds :type Float%20%28double-precision%29) (TriggeredSeconds :type Float%20%28double-precision%29) (InputAction :type Input%20Action%20Object%20Reference :default "/Game/Player/Blueprints/Input/IA_Sprint.IA_Sprint"))
  ;[0.15 0.15 0.15 0.5] Sprint Code
  (:Started
    (if (not (AI|Components|NavMovement|IsCrouching (Variables|Character|GetCharacterMovement)))
      (Variables|Components|SetIsSprinting true)
      (Variables|/Script/Engine.CharacterMovementComponent|SetMaxWalkSpeed (Variables|Character|GetCharacterMovement) (Variables|Components|GetSprintSpeed))))
  (:Completed
    (Variables|Components|SetIsSprinting false)
    (Variables|/Script/Engine.CharacterMovementComponent|SetMaxWalkSpeed (Variables|Character|GetCharacterMovement) (Variables|Components|GetWalkSpeed))))

(event Input|EnhancedActionEvents|EnhancedInputActionIA_Interact
  (params (ActionValue :type Boolean) (ElapsedSeconds :type Float%20%28double-precision%29) (TriggeredSeconds :type Float%20%28double-precision%29) (InputAction :type Input%20Action%20Object%20Reference :default "/Game/Player/Blueprints/Input/IA_Interact.IA_Interact"))
  (bind _currentinteractable (Variables|Interact|GetCurrentInteractable))
  (:Started
    (if (not (or (Variables|Interact|GetIsInspecting) (Variables|Interact|GetIsUsingKeypad)))
      (if (Variables|Interact|GetCanInteract)
        (Utilities|IsValid _currentinteractable
          (:Is%20Valid
            (Class|BPIInteractable|Interact(Message) _currentinteractable self)))))))

(event Input|EnhancedActionEvents|EnhancedInputActionIA_PhotoEvidence
  (params (ActionValue :type Boolean) (ElapsedSeconds :type Float%20%28double-precision%29) (TriggeredSeconds :type Float%20%28double-precision%29) (InputAction :type Input%20Action%20Object%20Reference :default "/Game/Player/Blueprints/Input/IA_PhotoEvidence.IA_PhotoEvidence"))
  (bind _inspectedobject (Variables|Inspect|GetInspectedObject))
  (bind _evidencedata (Variables|/Game/Blueprints/Interactables/BP_InspectableObject.BP_InspectableObject_C|GetEvidenceData _inspectedobject))
  (:Started
    (if (Variables|Interact|GetIsInspecting)
      (Utilities|IsValid _inspectedobject
        (:Is%20Valid
          (bind _wasadded (CallFunction|AddEvidence _evidencedata))
          (if _wasadded
            (Development|PrintString "Evidence Saved")
            (Development|PrintText (.ImportantInfo (Utilities|Struct|BreakS_EvidenceData _evidencedata)))
            (else
              (Development|PrintString "Evidence Already Saved")))))
      (else
        (Development|PrintString "Not Inspecting")))))

(event Input|EnhancedActionEvents|EnhancedInputActionIA_ExitInspect
  (params (ActionValue :type Boolean) (ElapsedSeconds :type Float%20%28double-precision%29) (TriggeredSeconds :type Float%20%28double-precision%29) (InputAction :type Input%20Action%20Object%20Reference :default "/Game/Player/Blueprints/Input/IA_ExitInspect.IA_ExitInspect"))
  (:Started
    (if (Variables|Interact|GetIsInspecting)
      (CallFunction|EndInspectingObject)
      (else
        (Development|PrintString "Not Inspecting")))))

(event EventBeginPlay
  (bind _returnvalue (Game|GetPlayerController 0))
  (Input|AddMappingContext (PlayerController|LocalPlayerSubsystems|GetEnhancedInputLocalPlayerSubsystem (Game|GetPlayerController 0)) "/Game/Player/Blueprints/Input/IMC_Player.IMC_Player" 0 "(bIgnoreAllPressedKeysUntilRelease=True,bForceImmediately=False,bNotifyUserSettings=False)")
  (bind _returnvalue_2 (UserInterface|CreateWidget "/Game/UI/WBP_InteractPrompt.WBP_InteractPrompt_C" _returnvalue))
  (bind _output_get (Variables|Interact|SetInteractPromptWidget _returnvalue_2))
  (UserInterface|Viewport|AddtoViewport _output_get 0)
  (Widget|SetVisibility _output_get "Hidden")
  (bind _returnvalue_3 (UserInterface|CreateWidget "/Game/UI/WBP_InspectInfo.WBP_InspectInfo_C" _returnvalue))
  (bind _output_get_2 (Variables|Inspect|SetInspectInfoWidget _returnvalue_3))
  (UserInterface|Viewport|AddtoViewport _output_get_2 0)
  (Widget|SetVisibility _output_get_2 "Collapsed")
  (Variables|Timer|SetTimeRemaining (Variables|Timer|GetStartingTime))
  (bind _returnvalue_4 (UserInterface|CreateWidget "/Game/UI/WBP_Timer.WBP_Timer_C" _returnvalue))
  (bind _output_get_3 (Variables|Timer|SetTimerWidget _returnvalue_4))
  (UserInterface|Viewport|AddtoViewport _output_get_3 0)
  (Default|UpdateTimerDisplay (Variables|Timer|GetTimerWidget) (Variables|Timer|GetTimeRemaining))
  (Utilities|Time|SetTimerbyFunctionName 0 "CountdownTick" 1.0 true))

(event Collision|EventActorBeginOverlap
  (params (OtherActor :type Actor%20Object%20Reference)))

(event EventTick
  (params (DeltaSeconds :type Float%20%28single-precision%29))
  ;[0.15 0.15 0.15 0.5] Player constantly checking what they are looking at and that they are walking.
  (Utilities|FlowControl|Sequence
    (:then_0
      (CallFunction|InteractionTrace))
    (:then_1
      (CallFunction|UpdateFootsteps DeltaSeconds))))

(fn ConstructionScript)

(fn InteractionTrace
  (bind _firstpersoncamera (Variables|Default|GetFirstPersonCamera))
  (bind _interactpromptwidget (Variables|Interact|GetInteractPromptWidget))
  (bind _returnvalue (Transformation|GetWorldLocation _firstpersoncamera))
  (if (or (Variables|Interact|GetIsInspecting) (Variables|Interact|GetIsUsingKeypad))
    (Variables|Interact|SetCurrentInteractable 0)
    (Variables|Interact|SetCanInteract false)
    (Widget|SetVisibility (Variables|Interact|GetInteractPromptWidget) "Hidden")
    (else
      (bind (_outhit _returnvalue_2) (Collision|LineTraceByChannel _returnvalue (+ _returnvalue (* (Math|Vector|GetForwardVector _firstpersoncamera) (Variables|Interact|GetTraceDistance))) "TraceTypeQuery1" false 0 "None"))
      (if _returnvalue_2
        (if (Utilities|DoesObjectImplementInterface (.HitActor (Collision|BreakHitResult _outhit)) "/Game/Player/Blueprints/Interfaces/BPI_Interactable.BPI_Interactable_C")
          (Variables|Interact|SetCurrentInteractable (.HitActor (Collision|BreakHitResult _outhit)))
          (Variables|Interact|SetCanInteract true)
          (bind _interacttext (Class|BPIInteractable|GetInteractText(Message) (.HitActor (Collision|BreakHitResult _outhit))))
          (Variables|/Script/UMG.TextBlock|SetText (Variables|/Game/UI/WBP_InteractPrompt.WBP_InteractPrompt_C|GetPromptText _interactpromptwidget) _interacttext)
          (Widget|SetVisibility _interactpromptwidget "Visible")
          (else
            (Widget|SetVisibility (Variables|Interact|GetInteractPromptWidget) "Hidden" :!label _label)))
        (else
          (Variables|Interact|SetCurrentInteractable 0)
          (Variables|Interact|SetCanInteract false)
          (goto _label))))))

(fn StartInspectingObject
  (params (ObjectToInspect :type BP%20Inspectable%20Object%20Object%20Reference))
  (bind _evidencedata (Variables|/Game/Blueprints/Interactables/BP_InspectableObject.BP_InspectableObject_C|GetEvidenceData ObjectToInspect))
  (bind _inspectinfowidget (Variables|Inspect|GetInspectInfoWidget))
  (bind (_evidencename _evidencedescription) (Utilities|Struct|BreakS_EvidenceData _evidencedata))
  (if (not (Variables|Interact|GetIsInspecting))
    (Variables|Interact|SetIsInspecting true)
    (Variables|Inspect|SetInspectedObject ObjectToInspect)
    (Variables|Inspect|SetInspectedObjectOriginalTransform (Transformation|GetActorTransform ObjectToInspect))
    (Components|Movement|StopMovementImmediately (Variables|Character|GetCharacterMovement))
    (Input|SetIgnoreMoveInput (Pawn|GetController) true)
    (Variables|Interact|SetCanInteract false)
    (Variables|Interact|SetCurrentInteractable 0)
    (Widget|SetVisibility (Variables|Interact|GetInteractPromptWidget) "Hidden")
    (Collision|SetActorEnableCollision ObjectToInspect false)
    (Transformation|AttachComponentToComponent ObjectToInspect (Variables|Default|GetFirstPersonCamera) "None" "SnapToTarget" "SnapToTarget" "KeepWorld" false)
    (Transformation|SetActorRelativeLocation ObjectToInspect (Variables|Inspect|GetInspectLocation))
    (Variables|Inspect|SetInspectYaw 0.0)
    (Variables|Inspect|SetInspectPitch 0.0)
    (Transformation|SetActorRelativeRotation ObjectToInspect (Variables|Inspect|GetInspectRotation))
    (Default|UpdateInspectInfo _inspectinfowidget _evidencename _evidencedescription)
    (Widget|SetVisibility _inspectinfowidget "Visible")
    (Camera|SetFieldOfView (Variables|Default|GetFirstPersonCamera) (Variables|Components|GetInspectFOV))))

(fn EndInspectingObject
  (if (Variables|Interact|GetIsInspecting)
    (Utilities|IsValid (Variables|Inspect|GetInspectedObject)
      (:Is%20Valid
        (Transformation|DetachFromActor (Variables|Inspect|GetInspectedObject) "KeepWorld" "KeepWorld" "KeepWorld")
        (Transformation|SetActorTransform (Variables|Inspect|GetInspectedObject) (Variables|Inspect|GetInspectedObjectOriginalTransform))
        (Collision|SetActorEnableCollision (Variables|Inspect|GetInspectedObject) true)
        (Input|SetIgnoreMoveInput (Pawn|GetController) false)
        (Variables|Interact|SetIsInspecting false)
        (Variables|Inspect|SetInspectedObject 0)
        (Widget|SetVisibility (Variables|Inspect|GetInspectInfoWidget) "Collapsed")
        (Camera|SetFieldOfView (Variables|Default|GetFirstPersonCamera) (Variables|Components|GetNormalFOV))))))

(fn AddEvidence
  (params (NewEvidence :type S%20Evidence%20Data%20Structure))
  (bind _evidenceinventory (Variables|Interact|GetEvidenceInventory))
  (if (== (.EvidenceID (Utilities|Struct|BreakS_EvidenceData NewEvidence)) "")
    (Development|PrintString "EvidenceID is Empty")
    (return false)
    (else
      (for _array_element _evidenceinventory
        (if (== (.EvidenceID (Utilities|Struct|BreakS_EvidenceData _array_element)) (.EvidenceID (Utilities|Struct|BreakS_EvidenceData NewEvidence)))
          (return false)))
      (Utilities|Array|Add _evidenceinventory NewEvidence)
      (Audio|PlaySound2D "/Game/Audio/SFX/UI/SFX_UI_Success.SFX_UI_Success" 1.0 1.0 0.0 0 0)
      (return true))))

(fn CountdownTick
  (bind _musiccomponent (Variables|Default|GetMusicComponent))
  (bind _output_get (Variables|Timer|SetTimeRemaining (- (Variables|Timer|GetTimeRemaining) 1)))
  (Default|UpdateTimerDisplay (Variables|Timer|GetTimerWidget) _output_get)
  (if (<= (Variables|Timer|GetTimeRemaining) 0)
    (CallFunction|GameOver)
    (elif (== (Variables|Timer|GetTimeRemaining) 60)
      (Audio|Components|Audio|SetVolumeMultiplier _musiccomponent 0.65 :!class /Script/Engine.AudioComponent)
      (Audio|Components|Audio|SetPitchMultiplier _musiccomponent 1.05))))

(fn PlayFootstep
  (Audio|PlaySoundatLocation (Variables|Audio|GetFootstepSound) (Transformation|GetActorLocation) "0, 0, 0" 1.0 1.0 0.0 0 0 0 0))

(fn UpdateFootsteps
  (params (DeltaSeconds :type Float%20%28double-precision%29))
  (if (and (> (Math|Vector|VectorLengthXY (Transformation|GetVelocity)) 1e+01) (AI|Components|NavMovement|IsMovingonGround (Variables|Character|GetCharacterMovement)))
    (bind _output_get (Variables|Audio|SetFootstepElapsed (+ (Variables|Audio|GetFootstepElapsed) DeltaSeconds)))
    (if (>= _output_get (Variables|Audio|GetFootstepInterval))
      (CallFunction|PlayFootstep)
      (Variables|Audio|SetFootstepElapsed 0.0))
    (else
      (Variables|Audio|SetFootstepElapsed 0.0))))