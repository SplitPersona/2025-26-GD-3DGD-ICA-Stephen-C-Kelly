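; BP_LockedDoor is an interactable hinged door that can be locked, swinging open or closed when used.
; Interact plays a locked sound while locked, otherwise toggles the door with open or close sounds.
; A timeline played forward or reversed lerps the pivot between the closed rotation captured at BeginPlay and a yaw-offset open rotation.
; UnlockDoor clears the lock, and GetInteractText returns a prompt matching the current state.
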(event Custom|ToggleDoor
  (bind _returnvalue (Transformation|GetActorLocation))
  (if (Variables|Default|GetIsOpen)
    (Variables|Default|SetIsOpen false)
    (Audio|PlaySoundatLocation (Variables|Audio|GetCloseSound) _returnvalue "0, 0, 0" 1.0 1.0 0.0 "/Game/Audio/Attenuation/ATT_3D_Medium.ATT_3D_Medium" 0 0 0)
    (bind _alpha (Timeline|TL_DoorOpen Reverse)
      (:Update
        (Transformation|SetRelativeRotation (Variables|Default|GetDoorPivot) (Math|Rotator|Lerp(Rotator) (Variables|Default|GetClosedRotation) (Variables|Default|GetOpenRotation) _alpha) false false)))
    (else
      (Variables|Default|SetIsOpen true)
      (Audio|PlaySoundatLocation (Variables|Audio|GetOpenSound) _returnvalue "0, 0, 0" 1.0 1.0 0.0 "/Game/Audio/Attenuation/ATT_3D_Medium.ATT_3D_Medium" 0 0 0)
      (Timeline|TL_DoorOpen Play))))

(event EventBeginPlay
  (bind _doorpivot (Variables|Default|GetDoorPivot))
  (bind _relativerotation (Variables|/Script/Engine.SceneComponent|GetRelativeRotation _doorpivot))
  (bind (_roll _pitch _yaw) (Math|Rotator|BreakRotator _relativerotation))
  (Variables|Default|SetClosedRotation _relativerotation)
  (Variables|Default|SetOpenRotation (Math|Rotator|MakeRotator _roll _pitch (+ _yaw (Variables|Default|GetOpenAngle)))))

(event Collision|EventActorBeginOverlap
  (params (OtherActor :type Actor%20Object%20Reference)))

(event EventTick
  (params (DeltaSeconds :type Float%20%28single-precision%29)))

(event EventInteract
  (params (PlayerRef :type BP%20Player%20Character%20Object%20Reference))
  (if (Variables|Default|GetIsLocked)
    (Audio|PlaySoundatLocation (Variables|Audio|GetLockedSound) (Transformation|GetActorLocation) "0, 0, 0" 1.0 1.0 0.0 "/Game/Audio/Attenuation/ATT_3D_Medium.ATT_3D_Medium" 0 0 0)
    (else
      (CallFunction|ToggleDoor))))

(fn ConstructionScript)

(fn UnlockDoor
  (Variables|Default|SetIsLocked false)
  (Development|PrintString "Door Unlocked"))

(fn GetInteractText
  (if (Variables|Default|GetIsLocked)
    (return (Variables|Default|GetLockedText))
    (elif (Variables|Default|GetIsOpen)
      (return (Variables|Default|GetCloseText))
      (else
        (return (Variables|Default|GetOpenText))))))