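; BP_Drawer is an interactable drawer that slides open and closed, carrying any contained evidence with it.
; On BeginPlay it records closed and open positions along local X from OpenDistance and attaches ContainedEvidence to DrawerRoot, keeping world transform.
; Interact toggles IsOpen and plays or reverses the TL_Drawer timeline, which lerps DrawerRoot's relative location.
; GetInteractText returns an open or close prompt matching the current state.
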(event Custom|ToggleDrawer
  (if (Variables|Interaction|GetIsOpen)
    (Variables|Interaction|SetIsOpen false)
    (bind _alpha (Timeline|TL_Drawer Reverse)
      (:Update
        (Transformation|SetRelativeLocation (Variables|Default|GetDrawerRoot) (Math|Vector|Lerp(Vector) (stale EventBeginPlay _output_get) (stale EventBeginPlay _output_get_2) _alpha) false false)))
    (else
      (Variables|Interaction|SetIsOpen true)
      (Timeline|TL_Drawer Play))))

(event EventBeginPlay
  (bind _drawerroot (Variables|Default|GetDrawerRoot))
  (bind _containedevidence (Variables|Evidence|GetContainedEvidence))
  (bind _relativelocation (Variables|/Script/Engine.SceneComponent|GetRelativeLocation _drawerroot))
  (bind _output_get (Variables|Interaction|SetClosedLocation _relativelocation))
  (bind _output_get_2 (Variables|Interaction|SetOpenLocation (+ _relativelocation (Math|Vector|MakeVector (Variables|Interaction|GetOpenDistance) 0.0 0.0))))
  (Utilities|IsValid _containedevidence
    (:Is%20Valid
      (Transformation|AttachComponentToComponent _containedevidence (Variables|Default|GetDrawerRoot) "None" "KeepWorld" "KeepWorld" "KeepWorld" true))))

(event Collision|EventActorBeginOverlap
  (params (OtherActor :type Actor%20Object%20Reference)))

(event EventTick
  (params (DeltaSeconds :type Float%20%28single-precision%29)))

(event EventInteract
  (params (PlayerRef :type BP%20Player%20Character%20Object%20Reference))
  (CallFunction|ToggleDrawer))

(fn ConstructionScript)

(fn GetInteractText
  (if (Variables|Interaction|GetIsOpen)
    (return "Press E to Close Drawer")
    (else
      (return "Press E to Open Drawer"))))