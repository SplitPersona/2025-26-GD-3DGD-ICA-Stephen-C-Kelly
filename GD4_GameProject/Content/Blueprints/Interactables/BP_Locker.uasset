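; BP_Locker is an interactable locker whose door the player can open and close.
; Interact calls ToggleLocker, which flips IsOpen and plays or reverses the TL_LockerDoor timeline.
; The timeline lerps DoorPivot's relative rotation between the closed pose cached at BeginPlay and one offset in yaw by OpenAngle.
; GetInteractText returns an open or close prompt based on IsOpen.
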(event Custom|ToggleLocker
  (if (Variables|InteractVars|GetIsOpen)
    (Variables|InteractVars|SetIsOpen false)
    (bind _alpha (Timeline|TL_LockerDoor Reverse)
      (:Update
        (Transformation|SetRelativeRotation (Variables|Default|GetDoorPivot) (Math|Rotator|Lerp(Rotator) (Variables|InteractVars|GetClosedRotation) (Variables|InteractVars|GetOpenRotation) _alpha true) false false)))
    (else
      (Variables|InteractVars|SetIsOpen true)
      (Timeline|TL_LockerDoor Play))))

(event EventBeginPlay
  (bind _doorpivot (Variables|Default|GetDoorPivot))
  (bind _relativerotation (Variables|/Script/Engine.SceneComponent|GetRelativeRotation _doorpivot))
  (bind (_roll _pitch _yaw) (Math|Rotator|BreakRotator _relativerotation))
  (Variables|InteractVars|SetClosedRotation _relativerotation)
  (Variables|InteractVars|SetOpenRotation (Math|Rotator|MakeRotator _roll _pitch (+ _yaw (Variables|InteractVars|GetOpenAngle)))))

(event Collision|EventActorBeginOverlap
  (params (OtherActor :type Actor%20Object%20Reference)))

(event EventTick
  (params (DeltaSeconds :type Float%20%28single-precision%29)))

(event EventInteract
  (params (PlayerRef :type BP%20Player%20Character%20Object%20Reference))
  (CallFunction|ToggleLocker))

(fn ConstructionScript)

(fn GetInteractText
  (if (Variables|InteractVars|GetIsOpen)
    (return "Press E to Close Locker")
    (else
      (return "Press E to Open Locker"))))