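; BP_Keypad is an interactable code lock that, while powered, lets the player enter a code to unlock a linked door.
; Interacting creates a WBP_Keypad widget holding a reference back to the keypad, blocks movement and shows the cursor.
; Digits build a length-capped string pushed to the display, and submitting compares it to the correct code with sound feedback.
; A match unlocks and closes only if a linked door is valid, while a mismatch clears the entry.
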(event EventBeginPlay)

(event Collision|EventActorBeginOverlap
  (params (OtherActor :type Actor%20Object%20Reference)))

(event EventTick
  (params (DeltaSeconds :type Float%20%28single-precision%29)))

(event EventInteract
  (params (PlayerRef :type BP%20Player%20Character%20Object%20Reference))
  (if (Variables|Power|GetIsPowered)
    (CallFunction|OpenKeypad PlayerRef)
    (else
      (Development|PrintString "Keypad has no power"))))

(fn ConstructionScript)

(fn OpenKeypad
  (params (PlayerRef :type BP%20Player%20Character%20Object%20Reference))
  (bind _returnvalue (Game|GetPlayerController 0))
  (bind _output_get (Variables|Default|SetUsingPlayer PlayerRef))
  (Variables|Default|SetEnteredCode "")
  (Variables|/Game/Player/Blueprints/BP_PlayerCharacter.BP_PlayerCharacter_C|SetIsUsingKeypad _output_get true)
  (Widget|SetVisibility (Variables|/Game/Player/Blueprints/BP_PlayerCharacter.BP_PlayerCharacter_C|GetInteractPromptWidget _output_get) "Hidden")
  (bind _returnvalue_2 (UserInterface|CreateWidget "/Game/UI/WBP_Keypad.WBP_Keypad_C" _returnvalue self))
  (bind _output_get_2 (Variables|Default|SetKeypadWidget _returnvalue_2))
  (UserInterface|Viewport|AddtoViewport _output_get_2 0)
  (Variables|/Script/Engine.PlayerController|SetbShowMouseCursor _returnvalue true)
  (Input|SetInputModeGameandUI _returnvalue _output_get_2 "DoNotLock" true false)
  (Input|SetIgnoreMoveInput _returnvalue true))

(fn AddDigit
  (params (Digit :type String))
  (if (< (Utilities|String|Len (Variables|Default|GetEnteredCode)) (Variables|Default|GetMaxCodeLength))
    (Variables|Default|SetEnteredCode (Utilities|String|Append (Variables|Default|GetEnteredCode) Digit))
    (Audio|PlaySound2D (Variables|Audio|GetKeyBeepSound) 1.0 1.0 0.0 0 0)
    (CallFunction|UpdateKeypadDisplay)))

(fn UpdateKeypadDisplay
  (bind _keypadwidget (Variables|Default|GetKeypadWidget))
  (Utilities|IsValid _keypadwidget
    (:Is%20Valid
      (Default|UpdateDisplay _keypadwidget (Utilities|Text|ToText(String) (Variables|Default|GetEnteredCode))))))

(fn ClearCode
  (Variables|Default|SetEnteredCode "")
  (CallFunction|UpdateKeypadDisplay))

(fn SubmitCode
  (bind _linkeddoor (Variables|Default|GetLinkedDoor))
  (if (Utilities|Enum|Equal(Enum) (Variables|Default|GetEnteredCode) (Variables|Default|GetCorrectCode))
    (Audio|PlaySound2D (Variables|Audio|GetSuccessSound) 1.0 1.0 0.0 0 0)
    (Utilities|IsValid _linkeddoor
      (:Is%20Valid
        (Default|UnlockDoor _linkeddoor)
        (CallFunction|CloseKeypad)))
    (else
      (Audio|PlaySound2D (Variables|Audio|GetFailSound) 1.0 1.0 0.0 0 0)
      (CallFunction|ClearCode))))

(fn CloseKeypad
  (bind _returnvalue (Game|GetPlayerController 0))
  (bind _keypadwidget (Variables|Default|GetKeypadWidget))
  (bind _usingplayer (Variables|Default|GetUsingPlayer))
  (Utilities|IsValid _keypadwidget
    (:Is%20Valid
      (Widget|RemovefromParent _keypadwidget)
      (Utilities|IsValid _usingplayer
        (:Is%20Valid
          (Variables|/Game/Player/Blueprints/BP_PlayerCharacter.BP_PlayerCharacter_C|SetIsUsingKeypad _usingplayer false)
          (Input|SetIgnoreMoveInput _returnvalue false)
          (Variables|/Script/Engine.PlayerController|SetbShowMouseCursor _returnvalue false)
          (Input|SetInputModeGameOnly _returnvalue false)
          (CallFunction|ClearCode))))))

(fn GetInteractText
  (if (Variables|Power|GetIsPowered)
    (return (Variables|Default|GetInteractText))
    (else
      (return "No Power"))))