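; BP_PowerSwitch is an interactable, one-way switch that restores power to a linked keypad.
; On Interact it sets IsOn, then, if LinkedKeypad is valid, sets the keypad's IsPowered flag and plays a power-on sound at the switch.
; Later interactions only print an already-restored message.
; GetInteractText returns a restore prompt or a powered status based on IsOn.
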(event EventBeginPlay)

(event Collision|EventActorBeginOverlap
  (params (OtherActor :type Actor%20Object%20Reference)))

(event EventTick
  (params (DeltaSeconds :type Float%20%28single-precision%29)))

(event EventInteract
  (params (PlayerRef :type BP%20Player%20Character%20Object%20Reference))
  (bind _linkedkeypad (Variables|Interactable|GetLinkedKeypad))
  (if (Variables|Power|GetIsOn)
    (Development|PrintString "Power alrady restored")
    (else
      (Variables|Power|SetIsOn true)
      (Utilities|IsValid _linkedkeypad
        (:Is%20Valid
          (Variables|/Game/Blueprints/Interactables/BP_Keypad.BP_Keypad_C|SetIsPowered _linkedkeypad true)
          (Audio|PlaySoundatLocation (Variables|Audio|GetPowerOnSound) (Transformation|GetActorLocation) "0, 0, 0" 1.0 1.0 0.0 "/Game/Audio/Attenuation/ATT_3D_Medium.ATT_3D_Medium" 0 0 0))))))

(fn ConstructionScript)

(fn GetInteractText
  (if (Variables|Power|GetIsOn)
    (return "Power On")
    (else
      (return "Press E to Restore Power"))))