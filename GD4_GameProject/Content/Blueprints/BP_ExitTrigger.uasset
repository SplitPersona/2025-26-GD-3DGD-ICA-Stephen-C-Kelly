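; BP_ExitTrigger is the level exit that ends play with an escape screen when the player reaches it.
; The ExitTrigger component's begin overlap casts to BP_PlayerCharacter and passes a DoOnce, so the sequence fires only once.
; It stops the character's movement, ignores move and look input, then shows WBP_YouEscaped with the mouse cursor and UI-only input.
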(event OnComponentBeginOverlap(ExitTrigger)
  (params (OverlappedComponent :type Primitive%20Component%20Object%20Reference) (OtherActor :type Actor%20Object%20Reference) (OtherComp :type Primitive%20Component%20Object%20Reference) (OtherBodyIndex :type Integer) (bFromSweep :type Boolean) (SweepResult :type Hit%20Result%20Structure%20%28by%20ref%29))
  (bind _returnvalue (Game|GetPlayerController 0))
  (bind _asbp_player_character (Utilities|Casting|CastToBP_PlayerCharacter OtherActor))
  (Utilities|FlowControl|DoOnce false
    (:Completed
      (Components|Movement|StopMovementImmediately (Variables|/Script/Engine.Character|GetCharacterMovement _asbp_player_character))
      (Input|SetIgnoreMoveInput (Pawn|GetController _asbp_player_character) true)
      (Input|SetIgnoreLookInput (Pawn|GetController _asbp_player_character) true)
      (bind _returnvalue_2 (UserInterface|CreateWidget "/Game/UI/WBP_YouEscaped.WBP_YouEscaped_C" _returnvalue))
      (UserInterface|Viewport|AddtoViewport _returnvalue_2 100)
      (Variables|/Script/Engine.PlayerController|SetbShowMouseCursor _returnvalue true)
      (Input|SetInputModeUIOnly _returnvalue _returnvalue_2 "DoNotLock" false))))

(event EventBeginPlay)

(event Collision|EventActorBeginOverlap
  (params (OtherActor :type Actor%20Object%20Reference)))

(event EventTick
  (params (DeltaSeconds :type Float%20%28single-precision%29)))

(fn ConstructionScript)